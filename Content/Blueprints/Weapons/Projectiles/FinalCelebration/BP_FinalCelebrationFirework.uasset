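; BP_FinalCelebrationFirework is a firework launcher that fires shell projectiles for the final celebration.
; Its LaunchShell event spawns a BP_FinalCelebrationFireworkShell at the Arrow component, offsetting the arrow's rotation by a random angle within RandomAngle on each axis.
; It passes the requested color, a randomly picked burst particle system, and its motion, timing, smoke and sparkle settings through to the half-scale shell.
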(event Custom|LaunchShell
  (params (Firework%20Color :type Linear%20Color%20Structure))
  (bind _arrow (Variables|Default|GetArrow))
  (bind _burstparticlesystems (Variables|BurstProperties|GetBurstParticleSystems))
  (bind _returnvalue (Transformation|GetWorldTransform _arrow))
  (bind (_location _rotation) (Math|Transform|BreakTransform _returnvalue))
  ;[1 1 1] Launch the shell!
  (Game|SpawnActorfromClass "/Game/Blueprints/Weapons/Projectiles/FinalCelebration/BP_FinalCelebrationFireworkShell.BP_FinalCelebrationFireworkShell_C" (Math|Transform|MakeTransform _location (Math|Rotator|CombineRotators _rotation (Math|Rotator|MakeRotator (Math|Random|RandomFloatinRange (* (Variables|ShellProperties|GetRandomAngle) -1.0) (Variables|ShellProperties|GetRandomAngle)) (Math|Random|RandomFloatinRange (* (Variables|ShellProperties|GetRandomAngle) -1.0) (Variables|ShellProperties|GetRandomAngle)) (Math|Random|RandomFloatinRange (* (Variables|ShellProperties|GetRandomAngle) -1.0) (Variables|ShellProperties|GetRandomAngle)))) "0.500000,0.500000,0.500000") "AlwaysSpawn" 0 (Variables|ShellProperties|GetMaxRotationSpeed) (Variables|ShellProperties|GetMinRotationSpeed) (Variables|ShellProperties|GetMaxLaunchVelocity) (Variables|ShellProperties|GetMinLaunchVelocity) (Variables|ShellProperties|GetShellMaxLife) (Variables|ShellProperties|GetShellminLife) (Variables|BurstProperties|GetMaxBurstTime) (Variables|BurstProperties|GetMinBurstTime) (Utilities|Array|Get(acopy) _burstparticlesystems (Math|Random|RandomInteger (Utilities|Array|Length _burstparticlesystems))) Firework%20Color (Variables|ShellProperties|GetShellParticleSystem) (Variables|ShellProperties|GetFlareColor) (Variables|ShellProperties|GetShellTailColor) (Variables|ShellProperties|GetUseShellSmoke) (Variables|BurstProperties|GetUseBurstSmoke) (Variables|BurstProperties|GetBurstSparkleMultiplier) (Variables|ShellProperties|GetShellSparkleMultiplier) (Variables|BurstProperties|GetBurstStarMultiplier) 0) ; Spawn a shell projectile and pass settings through
)

(fn ConstructionScript)